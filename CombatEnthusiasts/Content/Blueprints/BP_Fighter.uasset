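; BP_Fighter is a player-controlled fighter with basic Enhanced Input movement.
; On BeginPlay it casts its controller to BP_PlayerController and adds an input mapping context to that player's Enhanced Input subsystem.
; IA_Movement stores its value in MovementInput, passes only the X axis to AddMovement, and zeroes the stored value on cancel or completion.
; Tick prints the stored X value every frame as debug output.
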(event `self.ReceiveBeginPlay`
  (bind _asbp_player_controller (cast `/Game/Blueprints/BP_PlayerController` (`self.GetController`)))
  (`EnhancedInputSubsystemInterface.AddMappingContext` (pcsubsystem `EnhancedInputLocalPlayerSubsystem` _asbp_player_controller) "/Game/Input/InputMappingContext.InputMappingContext" 0 (struct)))

(event `EnhancedInput|/Game/Input/IA_Movement`
  (params (ActionValue :type "Vector2D Structure") (ElapsedSeconds :type "Float (double-precision)") (TriggeredSeconds :type "Float (double-precision)") (InputAction :type "InputAction Object Reference" :default "/Game/Input/IA_Movement.IA_Movement"))
  (:`Triggered`
    (bind _output_get (set `self.Movement Input` ActionValue))
    (`self.AddMovement` (`KismetMathLibrary.BreakVector2D` _output_get)))
  (:`Canceled`
    (set `self.Movement Input` (0.0 0.0) :!label _label))
  (:`Completed`
    (goto _label)))

(event `self.ReceiveTick`
  (params (DeltaSeconds :type "Float (single-precision)"))
  (bind _movement_input_x (`KismetMathLibrary.BreakVector2D` (`self.Movement Input`)))
  (`KismetSystemLibrary.PrintString` (`KismetStringLibrary.Conv_DoubleToString` _movement_input_x)))

(fn `UserConstructionScript`)