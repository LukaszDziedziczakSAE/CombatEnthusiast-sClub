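; BP_FighterController is a controller that turns player input into commands on a Fighter character.
; On BeginPlay it adds the Enhanced Input mapping context, printing an error if the input subsystem is invalid.
; Input actions forward movement, run, block, kick and punch to the Fighter after a validity check, clearing held states on release.
; Kick and punch share one BeginAttack call, distinguished by index.
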(event `self.ReceiveBeginPlay`
  (bind _returnvalue (subsystem `EnhancedInputLocalPlayerSubsystem`))
  (`parent.ReceiveBeginPlay`)
  (`/Engine/EditorBlueprintResources/StandardMacros.IsValid` _returnvalue
    (:`Is Valid`
      (`EnhancedInputSubsystemInterface.AddMappingContext` _returnvalue "/Game/Input/InputMappingContext.InputMappingContext" 0 (struct)))
    (:`Is Not Valid`
      (`KismetSystemLibrary.PrintString` "Input Subsystem Invalid" true true (struct :`R` 1.0 :`G` 0.027672 :`B` 0.107347 :`A` 1.0) 60.0))))

(event `EnhancedInput|/Game/Input/IA_Movement`
  (params (ActionValue :type "Vector2D Structure") (ElapsedSeconds :type "Float (double-precision)") (TriggeredSeconds :type "Float (double-precision)") (InputAction :type "InputAction Object Reference" :default "/Game/Input/IA_Movement.IA_Movement"))
  (:`Triggered`
    (bind _fighter (`self.Fighter`)
      (:`then`
        (`Fighter.SetMovementInput` _fighter ActionValue))
      (:`else`)))
  (:`Completed`
    (bind _fighter_2 (`self.Fighter`)
      (:`then`
        (`Fighter.SetMovementInput` _fighter_2 (0.0 0.0)))
      (:`else`))))

(event `EnhancedInput|/Game/Input/IA_Run`
  (params (ActionValue :type Boolean) (ElapsedSeconds :type "Float (double-precision)") (TriggeredSeconds :type "Float (double-precision)") (InputAction :type "InputAction Object Reference" :default "/Game/Input/IA_Run.IA_Run"))
  (:`Triggered`
    (bind _fighter (`self.Fighter`)
      (:`then`
        (`Fighter.SetIsRunning` _fighter true))
      (:`else`)))
  (:`Completed`
    (bind _fighter_2 (`self.Fighter`)
      (:`then`
        (`Fighter.SetIsRunning` _fighter_2 false))
      (:`else`))))

(event `EnhancedInput|/Game/Input/IA_Block`
  (params (ActionValue :type Boolean) (ElapsedSeconds :type "Float (double-precision)") (TriggeredSeconds :type "Float (double-precision)") (InputAction :type "InputAction Object Reference" :default "/Game/Input/IA_Block.IA_Block"))
  (:`Triggered`
    (bind _fighter (`self.Fighter`)
      (:`then`
        (`Fighter.SetIsBlocking` _fighter true))
      (:`else`)))
  (:`Completed`
    (bind _fighter_2 (`self.Fighter`)
      (:`then`
        (`Fighter.SetIsBlocking` _fighter_2 false))
      (:`else`))))

(event `EnhancedInput|/Game/Input/IA_Kick`
  (params (ActionValue :type Boolean) (ElapsedSeconds :type "Float (double-precision)") (TriggeredSeconds :type "Float (double-precision)") (InputAction :type "InputAction Object Reference" :default "/Game/Input/IA_Kick.IA_Kick"))
  (:`Triggered`
    (bind _fighter (`self.Fighter`)
      (:`then`
        (`Fighter.BeginAttack` _fighter 0))
      (:`else`))))

(event `EnhancedInput|/Game/Input/IA_Punch`
  (params (ActionValue :type Boolean) (ElapsedSeconds :type "Float (double-precision)") (TriggeredSeconds :type "Float (double-precision)") (InputAction :type "InputAction Object Reference" :default "/Game/Input/IA_Punch.IA_Punch"))
  (:`Triggered`
    (bind _fighter (`self.Fighter`)
      (:`then`
        (`Fighter.BeginAttack` _fighter 1))
      (:`else`))))

(fn `UserConstructionScript`)